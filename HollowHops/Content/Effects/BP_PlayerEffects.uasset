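; Player effects component for BP_MainCharacter that applies a staged degradation debuff when health is low and Vul is high.
; A looping half-second timer averages both stats' distances from 50 to pick a phase.
; Phases 1 and 2 slow movement and drain health, with phase 2 also showing the WBP_SecondDegPhase overlay.
; Phase 3 only prints a debug message, then restores speed and removes the overlay like phase 0.
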(event EventBeginPlay
  (bind _returnvalue (Components|GetOwner))
  (Utilities|IsValid _returnvalue
    (:Is%20Valid
      (bind _asbp_main_character (Utilities|Casting|CastToBP_MainCharacter _returnvalue))
      (Variables|Default|SetOwnerCharacter _asbp_main_character)
      (bind _returnvalue_2 (UserInterface|CreateWidget "/Game/Widgets/WBP_SecondDegPhase.WBP_SecondDegPhase_C"))
      (Variables|Default|SetWidgetSecondPhaseDeg _returnvalue_2)
      (bind _returnvalue_3 (Utilities|Time|SetTimerbyFunctionName 0 "CheckAllEffects" 0.5 true))
      (Variables|Default|SetEffectUpdateTimerHandle _returnvalue_3)
      (Development|PrintString "Effects Component Initialized"))
    (:Is%20Not%20Valid
      (Development|PrintString "ERROR" true true "(R=1.000000,G=0.000000,B=0.074347,A=1.000000)"))))

(event EventTick
  (params (DeltaSeconds :type Float%20%28single-precision%29)))

(fn CheckAllEffects
  (if (Utilities|IsValid (Variables|Default|GetOwnerCharacter))
    (Development|PrintString "Checking effects...")
    (bind (_stacks _hp _vul _deviation) (CallFunction|CheckDegradationConditions))
    (CallFunction|ApplyDegradationEffects _stacks)
    (Development|PrintString (Utilities|String|Append "PHASE: " (Utilities|String|ToString(Integer) _stacks) "HP: " (Utilities|String|ToString(Float) _hp) "Vul:" (Utilities|String|ToString(Float) _vul) "Dev: " (Utilities|String|ToString(Float) _deviation)) true true "(R=0.000000,G=0.000000,B=0.000000,A=1.000000)")))

(fn CheckDegradationConditions
  (bind _ownercharacter (Variables|Default|GetOwnerCharacter))
  (bind _ownercharacter_2 (Variables|Default|GetOwnerCharacter))
  (bind _ownercharacter_3 (Variables|Default|GetOwnerCharacter))
  (bind _vul (Variables|/Game/MainCharacter/BP_MainCharacter.BP_MainCharacter_C|GetVul _ownercharacter))
  (bind _currenthealth (Variables|/Game/MainCharacter/BP_MainCharacter.BP_MainCharacter_C|GetCurrentHealth _ownercharacter))
  (if (Utilities|IsValid (Variables|Default|GetOwnerCharacter))
    (if (and (< (Variables|/Game/MainCharacter/BP_MainCharacter.BP_MainCharacter_C|GetCurrentHealth _ownercharacter_3) 5e+01) (> (Variables|/Game/MainCharacter/BP_MainCharacter.BP_MainCharacter_C|GetVul _ownercharacter_3) 5e+01))
      (bind _output_get (LocalVariables|SetHP_Diff (Math|Float|Absolute(Float) (- 5e+01 (Variables|/Game/MainCharacter/BP_MainCharacter.BP_MainCharacter_C|GetCurrentHealth _ownercharacter_2)))))
      (bind _output_get_2 (LocalVariables|SetVul_Diff (Math|Float|Absolute(Float) (- 5e+01 (Variables|/Game/MainCharacter/BP_MainCharacter.BP_MainCharacter_C|GetVul _ownercharacter_2)))))
      (bind _output_get_3 (LocalVariables|SetDev (/ (+ _output_get _output_get_2) 2.0)))
      (if (> _output_get_3 3e+01)
        (bind _output_get_4 (LocalVariables|SetTargetStacks 3))
        (return _output_get_4 _currenthealth _vul (LocalVariables|GetDev))
        (elif (> _output_get_3 15.0)
          (bind _output_get_5 (LocalVariables|SetTargetStacks 2))
          (return _output_get_5 _currenthealth _vul (LocalVariables|GetDev))
          (else
            (bind _output_get_6 (LocalVariables|SetTargetStacks 1))
            (return _output_get_6 _currenthealth _vul (LocalVariables|GetDev)))))
      (else
        (Development|PrintString "PHASE 0" true true "(R=0.312500,G=0.000000,B=0.013437,A=1.000000)" 0.5)))
    (else
      (Development|PrintString "ERROR. character not found"))))

(fn ApplyDegradationEffects
  (params (Stacks :type Integer))
  (bind _ownercharacter (Variables|Default|GetOwnerCharacter))
  (switch int Stacks
    (:0
      (Development|PrintString "NO EFFECT" true true "(R=0.046550,G=1.000000,B=0.000000,A=1.000000)")
      (Variables|/Script/Engine.CharacterMovementComponent|SetMaxWalkSpeed (Variables|/Script/Engine.Character|GetCharacterMovement _ownercharacter) (Variables|/Game/MainCharacter/BP_MainCharacter.BP_MainCharacter_C|GetNormalSpeed _ownercharacter) :!label _label)
      (Utilities|IsValid (Variables|Default|GetWidgetSecondPhaseDeg) :!label _label_2
        (:Is%20Valid
          (Development|PrintString "remove" true true "(R=1.000000,G=0.010976,B=0.000000,A=1.000000)")
          (Widget|RemovefromParent (Variables|Default|GetWidgetSecondPhaseDeg))
          (Variables|Default|SetIsAlreadyAdd false))))
    (:1
      (CallFunction|MinusSpeedtoFirstPhaseDeg)
      (CallFunction|MinusHPbyFirstPhaseDeg)
      (goto _label_2))
    (:2
      (CallFunction|MinusSpeedtoFirstPhaseDeg)
      (CallFunction|MinusHPbyFirstPhaseDeg)
      (if (not (Variables|Default|GetIsAlreadyAdd))
        (UserInterface|Viewport|AddtoViewport (Variables|Default|GetWidgetSecondPhaseDeg) 0)
        (Variables|Default|SetIsAlreadyAdd true)))
    (:3
      (Development|PrintString "DEVASTATION" true true "(R=0.565104,G=0.011550,B=0.000000,A=1.000000)")
      (goto _label))))

(fn MinusSpeedtoFirstPhaseDeg
  (LocalVariables|SetCharMove (Variables|/Script/Engine.Character|GetCharacterMovement (Variables|Default|GetOwnerCharacter)))
  (Development|PrintString "-hp/sec 
-speed" true true "(R=0.259756,G=0.000000,B=1.000000,A=1.000000)")
  (Variables|/Script/Engine.CharacterMovementComponent|SetMaxWalkSpeed (LocalVariables|GetCharMove) 2.1e+02))

(fn MinusHPbyFirstPhaseDeg
  (bind _ownercharacter (Variables|Default|GetOwnerCharacter))
  (Development|PrintString "debugdebug")
  (bind _output_get (Variables|/Game/MainCharacter/BP_MainCharacter.BP_MainCharacter_C|SetCurrentHealth _ownercharacter (- (Variables|/Game/MainCharacter/BP_MainCharacter.BP_MainCharacter_C|GetCurrentHealth _ownercharacter) 0.125)))
  (Default|UpdateHealth (Variables|/Game/MainCharacter/BP_MainCharacter.BP_MainCharacter_C|GetWBP_Health (Variables|Default|GetOwnerCharacter)) _output_get))