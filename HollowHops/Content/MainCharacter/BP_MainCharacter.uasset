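; Player character with running, stamina-limited dashing, jumping, swimming, crouching, health and a vulnerability stat.
; Tick updates stamina, picks walk speed from movement state and BP_PlayerEffects' Degradation or Devastation, which also drain health, and pauses into WBP_Death at zero health.
; Timelines smooth health and vulnerability changes shown in WBP_Health, with number keys as test triggers; full vulnerability triggers health loss.
; Crouch lerps capsule height, and standing retries on a timer until a sphere trace clears.
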(event Custom|JumpInput
  ;[0.7591 1 0.4087 1 25] Функция логики прыжка
  (if (AI|Components|NavMovement|IsMovingonGround (Variables|Character|GetCharacterMovement))
    (Character|Jump)))

(event Custom|StartCrouch
  ;[0.07506 0.04013 1 1 42] КАСТОМНЫЕ ФУНКЦИИ ЛОГИКИ ПРИСЕДА И ВСТАВАНИЯ (ДЛЯ ПРОВЕРКИ ВОЗМОЖНОСТИ ВСТАВАНИЯ ИСПОЛЬЗУЕТСЯ ОТДЕЛЬНАЯ ФУНКЦИЯ TRYSTANDUP)
  ;;[1 0 0.4106] ПРИСЕСТЬ
  (if (Variables|Default|GetIsRunning)
    (Variables|Default|SetIsRunning false))
  (Variables|Default|SetIsCrouching true)
  (CallFunction|TestforTimelineDegSpeed))

(event Custom|UpdateDecreaseVul
  ;[1 1 1] [TEST] Уменьшение уязвимости на 10% при нажатии на "3"
  (Timeline|Timeline_0 PlayFromStart
    (:Update
      (CallFunction|DecreaseVul))))

(event Custom|UpdateIncreaseVul
  ;[1 1 1] [TEST] Увеличение уязвимости на 10% при нажатии на "4"
  (Timeline|Timeline_1 PlayFromStart
    (:Update
      (CallFunction|IncreaseVul))))

(event Custom|DecreaseHealthIfDeg
  ;[0 0 0] Уменьшение здоровья при эффекте "Деградация" (-1%HP/5sec)
  (if (Variables|/Game/Effects/BP_PlayerEffects.BP_PlayerEffects_C|GetIsDegradation (Variables|Default|GetPlayerEffects))
    (Utilities|FlowControl|Delay 5.0)
    (bind _output_get (Variables|Default|SetCurrentHealth (- (Variables|Default|GetCurrentHealth) 1.0)))
    (Default|UpdateHealth (Variables|Default|GetWBP_Health) _output_get)))

(event Custom|DecreaseHealthIfDevastation
  (if (Variables|/Game/Effects/BP_PlayerEffects.BP_PlayerEffects_C|GetIsDevastation (Variables|Default|GetPlayerEffects))
    (Utilities|FlowControl|Delay 1.1)
    (bind _output_get (Variables|Default|SetCurrentHealth (- (Variables|Default|GetCurrentHealth) 1.0)))
    (Default|UpdateHealth (Variables|Default|GetWBP_Health) _output_get)))

(event Custom|StopCrouch
  ;[0.07506 0.04013 1 1 42] КАСТОМНЫЕ ФУНКЦИИ ЛОГИКИ ПРИСЕДА И ВСТАВАНИЯ (ДЛЯ ПРОВЕРКИ ВОЗМОЖНОСТИ ВСТАВАНИЯ ИСПОЛЬЗУЕТСЯ ОТДЕЛЬНАЯ ФУНКЦИЯ TRYSTANDUP)
  ;;[0 1 0.03342] ВСТАТЬ
  ;;;[0 0 0 0.5] Проверка препятствий над головой
  (bind _returnvalue (Collision|SphereTraceByChannel (Transformation|GetActorLocation) (+ (* (+ (* (Components|Capsule|GetScaledCapsuleHalfHeight (Variables|Collision|GetCapsuleComponent)) 2.0) 1e+01) "0.000000,0.000000,1.000000") (Transformation|GetActorLocation self)) (Components|Capsule|GetScaledCapsuleRadius (Variables|Collision|GetCapsuleComponent)) "TraceTypeQuery1" false 0 "None"))
  (if _returnvalue
    (Utilities|Time|SetTimerbyFunctionName self "TryStandUp" 0.1 true)
    (else
      (Variables|Default|SetIsCrouching false)
      (CallFunction|StopCrouchTest))))

(event Custom|StartRunInput
  ;[1 0.7227 0 1 38] Функции бега
  ;;[1 1 1] Функция начала бега
  (if (not (Variables|Default|GetIsCrouching))
    (Variables|Default|SetIsRunning true)))

(event Custom|StopRunInput
  ;[1 0.7227 0 1 38] Функции бега
  ;;[1 1 1] Функция остановки бега
  (Variables|Default|SetIsRunning false))

(event Custom|TestForTimelineDegSpeed
  ;[1 1 1] Функции плавного приседа
  (bind _alpha (Timeline|Timeline_2 Play)
    (:Update
      (Components|Capsule|SetCapsuleHalfHeight (Variables|Collision|GetCapsuleComponent) (Math|Float|Lerp 8e+01 34.0 _alpha) true))))

(event Custom|StopCrouchTest
  ;[1 1 1] Функции плавного приседа
  (bind _alpha (Timeline|Timeline_2 Reverse)
    (:Update
      (Components|Capsule|SetCapsuleHalfHeight (Variables|Collision|GetCapsuleComponent) (Math|Float|Lerp 8e+01 34.0 _alpha) true))))

(event Custom|StartDash
  ;[1 0.2812 0.2812 1 42] Функция логики рывка и трата выносливости при нем (кастомный event + кастомная функция
  (if (not (Variables|Default|GetIsCrouching))
    (CallFunction|StartDashing)
    (Timeline|DashingTimeline PlayFromStart
      (:Finished
        (CallFunction|StopDashing)))))

(event Custom|UpdateIncreaseHealth
  ;[1 1 1] Плавное увеличение здоровья
  (Timeline|Timeline PlayFromStart
    (:Update
      (CallFunction|IncreaseHealth))))

(event Custom|UpdateDecreaseHealth
  ;[1 1 1] Функция для плавного уменьшения здоровья
  (Timeline|HealthTimeline PlayFromStart
    (:Update
      (CallFunction|DecreaseHealth))))

(event Input|EnhancedActionEvents|EnhancedInputActionIA_Swimming
  (params (ActionValue :type Float%20%28double-precision%29) (ElapsedSeconds :type Float%20%28double-precision%29) (TriggeredSeconds :type Float%20%28double-precision%29) (InputAction :type Input%20Action%20Object%20Reference :default "/Game/input/IA_Swimming.IA_Swimming"))
  (bind _returnvalue (Pawn|GetControlRotation :!class /Script/Engine.Pawn))
  ;[0 0.131 1 1 80] Плавание персонажа
  (if (AI|Components|NavMovement|IsSwimming (Variables|Character|GetCharacterMovement) :!class /Script/Engine.NavMovementComponent)
    (Pawn|Input|AddMovementInput (Math|Vector|GetUpVector _returnvalue) ActionValue false)
    (Transformation|SetActorRotation _returnvalue)))

(event EventBeginPlay
  (Utilities|FlowControl|Sequence
    (:then_0
      ;[0 1 0.39] Создание виджета и выведение его на экран
      (bind _returnvalue (UserInterface|CreateWidget "/Game/Widgets/WBP_Health.WBP_Health_C"))
      (bind _output_get (Variables|Default|SetWBP_Health _returnvalue))
      (UserInterface|Viewport|AddtoViewport _output_get 0))
    (:then_1
      (bind _returnvalue_2 (UserInterface|CreateWidget "/Game/Widgets/WBP_Death.WBP_Death_C"))
      (Variables|Default|SetWBP_Death _returnvalue_2))
    (:then_2
      (Variables|Default|SetPlayerEffects (Actor|GetComponentbyClass "/Game/Effects/BP_PlayerEffects.BP_PlayerEffects_C")))))

(event EventTick
  (params (DeltaSeconds :type Float%20%28single-precision%29))
  ;[1 0.1668 0] Проверки уровня здоровья, уязвимости и выносливости
  (CallFunction|CheckHealth)
  (CallFunction|CheckVul)
  (CallFunction|CheckStamin)
  (Variables|Default|SetBP_PlayerEffects 0)
  (CallFunction|CheckSpeed)
  (CallFunction|DecreaseHealthifDeg)
  (CallFunction|DecreaseHealthifDevastation))

(event Input|KeyboardEvents|1
  (params (Key :type Key%20Structure :default "None"))
  ;[1 1 1] [TEST]
  (:Pressed
    (CallFunction|UpdateDecreaseHealth)))

(event Input|KeyboardEvents|2
  (params (Key :type Key%20Structure :default "None"))
  ;[1 1 1] [TEST]
  (:Pressed
    (CallFunction|UpdateIncreaseHealth)))

(event Input|KeyboardEvents|3
  (params (Key :type Key%20Structure :default "None"))
  ;[1 1 1] [TEST]
  (:Pressed
    (CallFunction|UpdateIncreaseVul)))

(event Input|KeyboardEvents|4
  (params (Key :type Key%20Structure :default "None"))
  ;[1 1 1] [TEST]
  (:Pressed
    (CallFunction|UpdateDecreaseVul)))

(fn ConstructionScript)

(fn TryStandUp
  ;[1 0 0.03067 1 38] Функця для постоянной попытки встать из приседа с учетом возможных препятствий сверху
  (bind _returnvalue (Collision|SphereTraceByChannel (Transformation|GetActorLocation) (+ (* (+ (* (Components|Capsule|GetScaledCapsuleHalfHeight (Variables|Collision|GetCapsuleComponent)) 2.0) 1e+01) "0.000000,0.000000,1.000000") (Transformation|GetActorLocation self)) (Components|Capsule|GetScaledCapsuleRadius (Variables|Collision|GetCapsuleComponent)) "TraceTypeQuery1" false 0 "None"))
  (if (not _returnvalue)
    (Utilities|Time|ClearTimerbyFunctionName 0 "TryStandUp")
    (CallFunction|StopCrouch)))

(fn CheckHealth
  (Utilities|FlowControl|Sequence
    (:then_0
      (if (<= (Variables|Default|GetCurrentHealth) 0.0)
        (if (not (Variables|Default|GetIsDead))
          (Variables|Default|SetIsDead true)
          (Default|UpdateHealth (Variables|Default|GetWBP_Health) (Variables|Default|GetCurrentHealth))
          (UserInterface|Viewport|AddtoViewport (Variables|Default|GetWBP_Death) 0)
          (Game|SetGamePaused true)
          (bind _asplayer_controller (Utilities|Casting|CastToPlayerController (Pawn|GetController)))
          (Variables|/Script/Engine.PlayerController|SetbShowMouseCursor _asplayer_controller true))))
    (:then_2
      ;[1 1 1] Полная потеря здоровья при 100% уязвимости
      (bind _maxvul (CallFunction|CheckVul))
      (if _maxvul
        (Variables|Default|SetDamage 1e+02)
        (CallFunction|UpdateDecreaseHealth)))))

(fn CheckVul
  (if (>= (Variables|Default|GetVul) 1e+02)
    (return true)))

(fn CheckStamin
  ;[1 0.8075 0 1 53] Проверка бега и расход выносливости
  (if (Variables|Default|GetIsRunning)
    (bind _output_get (Variables|Default|SetCurrentStamina (Math|Float|Clamp(Float) (- (Variables|Default|GetCurrentStamina) (* (Variables|Default|GetStaminaDrainRate) (Utilities|Time|GetWorldDeltaSeconds))) 0.0 (Variables|Default|GetMaxStamina))))
    (Default|UpdateStamina (Variables|Default|GetWBP_Health) _output_get)
    (if (<= (Variables|Default|GetCurrentStamina) 0.0)
      (CallFunction|StopRunInput))
    (elif (< (Variables|Default|GetCurrentStamina) (Variables|Default|GetMaxStamina))
      (bind _output_get_2 (Variables|Default|SetCurrentStamina (Math|Float|Clamp(Float) (+ (Variables|Default|GetCurrentStamina) (* (Variables|Default|GetStaminaRegenRate) (Utilities|Time|GetWorldDeltaSeconds))) 0.0 (Variables|Default|GetMaxStamina))))
      (Default|UpdateStamina (Variables|Default|GetWBP_Health) _output_get_2))))

(fn StartDashing
  ;[0.5721 0.1144 1] Расчет выносливости при рывке
  (if (>= (Variables|Default|GetCurrentStamina) 5e+01)
    (Variables|Default|SetIsDashing true)
    (Variables|Default|SetCurrentStamina (Math|Float|Clamp(Float) (- (Variables|Default|GetCurrentStamina) 3e+01) 0.0 (Variables|Default|GetMaxStamina)))))

(fn GetDamagefromCollisia1
  (Variables|Default|SetDamageUnits 9)
  (CallFunction|ConvertUnitsDamage)
  (CallFunction|UpdateDecreaseHealth))

(fn DecreaseHealth
  (bind _output_get (Variables|Default|SetCurrentHealth (Math|Float|Clamp(Float) (Math|Interpolation|FInterpTo (Variables|Default|GetCurrentHealth) (- (Variables|Default|GetCurrentHealth) 5.0) (Utilities|Time|GetWorldDeltaSeconds) 1.0) 0.0 1e+02)))
  (Default|UpdateHealth (Variables|Default|GetWBP_Health) _output_get))

(fn IncreaseHealth
  (bind _output_get (Variables|Default|SetCurrentHealth (Math|Float|Clamp(Float) (Math|Interpolation|FInterpTo (Variables|Default|GetCurrentHealth) (+ (Variables|Default|GetCurrentHealth) 1e+01) (Utilities|Time|GetWorldDeltaSeconds) 1.0) 0.0 1e+02)))
  (Default|UpdateHealth (Variables|Default|GetWBP_Health) _output_get))

(fn DecreaseVul
  (bind _output_get (Variables|Default|SetVul (Math|Float|Clamp(Float) (Math|Interpolation|FInterpTo (Variables|Default|GetVul) (- (Variables|Default|GetVul) 1e+01) (Utilities|Time|GetWorldDeltaSeconds) 1.0) 0.0 1e+02)))
  (Default|UpdateVul (Variables|Default|GetWBP_Health) _output_get))

(fn IncreaseVul
  (Variables|Default|SetFinalDamage (* (Variables|Default|GetDamage) (+ (* (Variables|Default|GetVul) 0.01) 1.0)))
  (bind _output_get (Variables|Default|SetVul (Math|Float|Clamp(Float) (Math|Interpolation|FInterpTo (Variables|Default|GetVul) (+ (Variables|Default|GetVul) (* (Class|KismetMathLibrary|FFloor64 (/ (Variables|Default|GetDamage) 1e+01)) 5)) (Utilities|Time|GetWorldDeltaSeconds) 1.0) 0.0 1e+02)))
  (Default|UpdateVul (Variables|Default|GetWBP_Health) _output_get))

(fn [TEST]DecreaseHealthifVulMore50
  (if (and (> (Variables|Default|GetVul) 5e+01) (Variables|Default|GetMoreVul50))
    (bind _output_get (Variables|Default|SetCurrentHealth (- (Variables|Default|GetCurrentHealth) 5e+01)))
    (Variables|Default|SetMoreVul50 false)
    (Default|UpdateHealth (Variables|Default|GetWBP_Health) _output_get)))

(fn ConvertUnitsDamage
  (Variables|Default|SetDamage (* (/ (Variables|Default|GetDamageUnits) (Variables|Default|GetMaxHP)) 1e+02)))

(fn StopDashing
  (Variables|Default|SetIsDashing false))

(fn CheckSpeed
  (if (Variables|/Game/Effects/BP_PlayerEffects.BP_PlayerEffects_C|GetIsDegradation (Variables|Default|GetPlayerEffects))
    ;[0 0.1449 1] ДЕГРАДАЦИЯ
    (if (Variables|Default|GetIsRunning)
      (Variables|/Script/Engine.CharacterMovementComponent|SetMaxWalkSpeed (Variables|Character|GetCharacterMovement) 4.2e+02)
      (elif (Variables|Default|GetIsCrouching)
        (Variables|/Script/Engine.CharacterMovementComponent|SetMaxWalkSpeed (Variables|Character|GetCharacterMovement) 105.0)
        (elif (Variables|Default|GetIsDashing)
          (Variables|/Script/Engine.CharacterMovementComponent|SetMaxWalkSpeed (Variables|Character|GetCharacterMovement) 1.05e+03)
          (else
            (Variables|/Script/Engine.CharacterMovementComponent|SetMaxWalkSpeed (Variables|Character|GetCharacterMovement) 2.1e+02)))))
    (else
      ;[0 0.06228 1] ОПУСТОШЕНИЕ
      (if (Variables|/Game/Effects/BP_PlayerEffects.BP_PlayerEffects_C|GetIsDevastation (Variables|Default|GetPlayerEffects))
        (if (Variables|Default|GetIsCrouching)
          (Variables|/Script/Engine.CharacterMovementComponent|SetMaxWalkSpeed (Variables|Character|GetCharacterMovement) 6e+01)
          (elif (Variables|Default|GetIsDashing)
            (Variables|/Script/Engine.CharacterMovementComponent|SetMaxWalkSpeed (Variables|Character|GetCharacterMovement) 6e+02)
            (elif (Variables|Default|GetIsRunning)
              (Variables|Default|SetIsRunning false)
              (else
                (Variables|/Script/Engine.CharacterMovementComponent|SetMaxWalkSpeed (Variables|Character|GetCharacterMovement) 1.8e+02)))))
        (else
          ;[0 0.03146 0.5339] ДЕФОЛТ
          (if (Variables|Default|GetIsRunning)
            (Variables|/Script/Engine.CharacterMovementComponent|SetMaxWalkSpeed (Variables|Character|GetCharacterMovement) 6e+02)
            (elif (Variables|Default|GetIsCrouching)
              (Variables|/Script/Engine.CharacterMovementComponent|SetMaxWalkSpeed (Variables|Character|GetCharacterMovement) 1.5e+02)
              (elif (Variables|Default|GetIsDashing)
                (Variables|/Script/Engine.CharacterMovementComponent|SetMaxWalkSpeed (Variables|Character|GetCharacterMovement) 1.5e+03)
                (else
                  (Variables|/Script/Engine.CharacterMovementComponent|SetMaxWalkSpeed (Variables|Character|GetCharacterMovement) (Variables|Default|GetNormalSpeed)))))))))))