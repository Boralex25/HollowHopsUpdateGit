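; Player controller that routes Enhanced Input actions to the player pawn and BP_MainCharacter.
; BeginPlay adds IMC_Control and caches the character reference.
; Look drives controller yaw and pitch; Move follows control rotation, or switches to Flying and moves along the actor's up vector while IsClimbing is set.
; Jump, crouch, run and dash inputs are forwarded to the character's own functions.
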(event Input|EnhancedActionEvents|EnhancedInputActionIA_Look
  (params (ActionValue :type Vector%202D%20Structure) (ElapsedSeconds :type Float%20%28double-precision%29) (TriggeredSeconds :type Float%20%28double-precision%29) (InputAction :type Input%20Action%20Object%20Reference :default "/Game/input/IA_Look.IA_Look"))
  ;[1 0 0.6943 1 40] Поворот камеры
  (Pawn|Input|AddControllerYawInput (Game|Player|GetPlayerPawn 0) (.x ActionValue))
  (Pawn|Input|AddControllerPitchInput (Game|Player|GetPlayerPawn 0) (.y ActionValue)))

(event Input|EnhancedActionEvents|EnhancedInputActionIA_Move
  (params (ActionValue :type Vector%202D%20Structure) (ElapsedSeconds :type Float%20%28double-precision%29) (TriggeredSeconds :type Float%20%28double-precision%29) (InputAction :type Input%20Action%20Object%20Reference :default "/Game/input/IA_Move.IA_Move"))
  (bind _returnvalue (Pawn|GetControlRotation :!class /Script/Engine.Controller))
  ;[1 0.2291 0.9167 1 44] Движение
  (if (Variables|/Game/MainCharacter/BP_MainCharacter.BP_MainCharacter_C|GetIsClimbing (Variables|Default|GetMainChar))
    (Pawn|Input|AddMovementInput (Variables|Default|GetMainChar) "0, 0, 0" 1.0 false)
    (Pawn|Components|CharacterMovement|SetMovementMode (Variables|/Script/Engine.Character|GetCharacterMovement (Variables|Default|GetMainChar)) "MOVE_Flying" 0)
    (Pawn|Input|AddMovementInput (Variables|Default|GetMainChar) (Transformation|GetActorUpVector (Game|GetPlayerCharacter 0)) (.y ActionValue) false)
    (else
      ;;[0.4901 0 1 1 49] вперед/назад
      (Pawn|Input|AddMovementInput (Game|Player|GetPlayerPawn 0) (Math|Vector|GetRightVector (Math|Rotator|MakeRotator (.roll _returnvalue) 0.0 (.yaw _returnvalue))) (.x ActionValue) false)
      ;;[0.4561 0 1 1 54] влево/вправо
      (Pawn|Input|AddMovementInput (Game|Player|GetPlayerPawn 0) (Math|Vector|GetForwardVector (Math|Rotator|MakeRotator 0.0 0.0 (.yaw (Pawn|GetControlRotation :!class /Script/Engine.Controller)))) (.y ActionValue) false))))

(event EventBeginPlay
  ;[1 0 0.2262 1 35] Подключение IMC, начало действия
  (Utilities|Casting|CastToCharacter (Game|Player|GetPlayerPawn 0))
  (Input|AddMappingContext (PlayerController|LocalPlayerSubsystems|GetEnhancedInputLocalPlayerSubsystem) "/Game/input/IMC_Control.IMC_Control" 0 "(bIgnoreAllPressedKeysUntilRelease=True,bForceImmediately=False,bNotifyUserSettings=False)")
  (bind _asbp_main_character (Utilities|Casting|CastToBP_MainCharacter (Game|Player|GetPlayerPawn 0)))
  (Variables|Default|SetMainChar _asbp_main_character))

(event Input|ActionEvents|InputActionIA_Crouch
  (params (Key :type Key%20Structure :default "None"))
  (bind _returnvalue (Pawn|GetControlledPawn))
  ;[0.4022 0 1 1 22] Вызов Input'а, затем (в зависимости от состояния) вызов функции приседа (нажатие) или вставания (отпускание кнопки)
  (:Pressed
    (bind _asbp_main_character (Utilities|Casting|CastToBP_MainCharacter _returnvalue))
    (Default|StartCrouch _asbp_main_character))
  (:Released
    (bind _asbp_main_character_2 (Utilities|Casting|CastToBP_MainCharacter _returnvalue))
    (Default|StopCrouch _asbp_main_character_2)))

(event Input|ActionEvents|InputActionIA_Jump
  (params (Key :type Key%20Structure :default "None"))
  ;[0.7196 0 1 1 25] Вызов Input'а, затем вызов кастомной функции прыжка
  (:Pressed
    (bind _asbp_main_character (Utilities|Casting|CastToBP_MainCharacter (Pawn|GetControlledPawn)))
    (Default|JumpInput _asbp_main_character)))

(event Input|ActionEvents|InputActionIA_Run
  (params (Key :type Key%20Structure :default "None"))
  ;[0.1847 0 1 1 32] Вызов Input'а, а затем начало или остановка бега
  (:Pressed
    (bind _asbp_main_character (Utilities|Casting|CastToBP_MainCharacter (Pawn|GetControlledPawn)))
    (Default|StartRunInput _asbp_main_character))
  (:Released
    (bind _asbp_main_character_2 (Utilities|Casting|CastToBP_MainCharacter (Pawn|GetControlledPawn)))
    (Default|StopRunInput _asbp_main_character_2)))

(event Input|ActionEvents|InputActionIA_Dash
  (params (Key :type Key%20Structure :default "None"))
  ;[0.593 0 1 1 25] Вызов Input'а, затем логика рывка из кастомной функции
  (:Pressed
    (bind _asbp_main_character (Utilities|Casting|CastToBP_MainCharacter (Pawn|GetControlledPawn)))
    (Default|StartDash _asbp_main_character)))

(fn ConstructionScript)