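; Inventory component that stores items as an array of ItemID and quantity slots.
; On BeginPlay it caches the first BP_ItemDatabase actor, which AddItem queries for each item's MaxStack.
; AddItem tops up matching slots and appends any overflow as one uncapped slot, skipping the stack limit when the inventory is empty.
; RemoveItem drains matching slots, deleting smaller ones mid-loop and leaving exactly emptied ones at zero.
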(event EventBeginPlay
  (bind _outactors (Actor|GetAllActorsOfClass "/Game/Assets/BP_ItemDatabase.BP_ItemDatabase_C"))
  (Variables|Default|SetItemDatabase (Utilities|Array|Get(acopy) _outactors)))

(event EventTick
  (params (DeltaSeconds :type Float%20%28single-precision%29)))

(fn AddItem
  (params (ItemID :type E_ItemID%20Enum :default "NewEnumerator3") (Quantity :type Integer))
  (LocalVariables|SetRemainingAdd Quantity)
  (Variables|Default|SetDAItem (.Value (Utilities|Map|Find (Variables|/Game/Assets/BP_ItemDatabase.BP_ItemDatabase_C|GetItemMap (Variables|Default|GetItemDatabase)) ItemID)))
  (Variables|Default|SetMaxStack (Variables|/Game/Assets/DA_Item.DA_Item_C|GetMaxStack (Variables|Default|GetDAItem)))
  (if (== (Utilities|Array|Length (Variables|Default|GetInventoryItems)) 0)
    (bind _output_get (Variables|Default|SetUpdateSlot (Utilities|Struct|MakeS_ItemInstance ItemID Quantity)))
    (Utilities|Array|Add (Variables|Default|GetInventoryItems) _output_get)
    (return true)
    (else
      (for (_array_element _array_index) (Variables|Default|GetInventoryItems)
        (Development|PrintString "CHECK" true true "(R=0.000000,G=0.000000,B=0.000000,A=1.000000)" 1e+01)
        (if (Utilities|Enum|Equal(Enum) (.itemid _array_element) ItemID)
          (Variables|Default|SetCurrentQuantity (.quantity _array_element))
          (Variables|Default|SetNewQuantity (+ (Variables|Default|GetCurrentQuantity) (LocalVariables|GetRemainingAdd)))
          (if (<= (Variables|Default|GetNewQuantity) (Variables|Default|GetMaxStack))
            (Variables|Default|SetUpdateSlot (Utilities|Struct|MakeS_ItemInstance (.itemid _array_element) (Variables|Default|GetNewQuantity)))
            (Utilities|Array|SetArrayElem (Variables|Default|GetInventoryItems) _array_index (Variables|Default|GetUpdateSlot))
            (LocalVariables|SetRemainingAdd 0)
            (return true)
            (else
              (Variables|Default|SetUpdateSlot (Utilities|Struct|MakeS_ItemInstance (.itemid _array_element) (Variables|Default|GetMaxStack)))
              (Utilities|Array|SetArrayElem (Variables|Default|GetInventoryItems) _array_index (Variables|Default|GetUpdateSlot))
              (LocalVariables|SetRemainingAdd (- (Variables|Default|GetNewQuantity) (Variables|Default|GetMaxStack)))
              (Development|PrintString "OVERFLOW" true true "(R=0.575521,G=0.503247,B=0.000000,A=1.000000)")))))
      (if (> (LocalVariables|GetRemainingAdd) 0)
        (bind _output_get_2 (Variables|Default|SetUpdateSlot (Utilities|Struct|MakeS_ItemInstance ItemID (LocalVariables|GetRemainingAdd))))
        (Utilities|Array|Add (Variables|Default|GetInventoryItems) _output_get_2)))))

(fn RemoveItem
  (params (InputItemID :type E_ItemID%20Enum :default "NewEnumerator3") (QuantityRemove :type Integer))
  (LocalVariables|SetRemainingToRemove QuantityRemove)
  (for (_array_element _array_index) (Variables|Default|GetInventoryItems)
    (if (Utilities|Enum|Equal(Enum) (.itemid _array_element) InputItemID)
      (if (>= (.quantity _array_element) (LocalVariables|GetRemainingToRemove))
        (bind _output_get (LocalVariables|SetUpdatedSlot (Utilities|Struct|MakeS_ItemInstance (.itemid _array_element) (- (.quantity _array_element) (LocalVariables|GetRemainingToRemove)))))
        (Utilities|Array|SetArrayElem (Variables|Default|GetInventoryItems) _array_index _output_get)
        (return true)
        (else
          (LocalVariables|SetRemainingToRemove (- (LocalVariables|GetRemainingToRemove) (.quantity _array_element)))
          (Utilities|Array|RemoveIndex (Variables|Default|GetInventoryItems) _array_index)))))
  (if (<= (LocalVariables|GetRemainingToRemove) 0)
    (return true)
    (else
      (return false))))